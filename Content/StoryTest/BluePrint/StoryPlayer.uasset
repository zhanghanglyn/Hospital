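; StoryPlayer plays a scripted story page by page through a level sequence player.
; OnClickNext calls PlayNext and plays the sequence, PlayOver stops it, and InitUI creates the StoryControl widget with a back-reference to the player.
; The startup chain (find first-person character, build UI, load scenario, start run) is unwired, as is look input, so BeginPlay only deactivates the root component.
; Debug prints remain.
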(event `InitUI`
  (bind _returnvalue (`GameplayStatics.GetPlayerController` 0))
  ;[1 1 1] UI逻辑
  (bind _returnvalue_2 (`|GenericCreateObject` "/Game/StoryTest/UI/StoryControl.StoryControl_C" self))
  (bind _output_get (set `self.StoryControl` _returnvalue_2))
  (set `/Game/StoryTest/UI/StoryControl.StoryPlayer` self _output_get)
  (`UserWidget.AddToViewport` _output_get 0)
  (`WidgetBlueprintLibrary.SetInputMode_UIOnlyEx` _returnvalue _output_get)
  (`WidgetBlueprintLibrary.SetInputMode_GameOnly` _returnvalue))

(event `self.ReceiveBeginPlay`
  (`ActorComponent.Deactivate` (`self.DefaultSceneRoot`)))

(event `OnClickNext`
  (bind _m_sequenceplayer (`self.m_sequencePlayer`))
  ;[1 1 1] 点击开始下一页
  (bind _returnvalue (`self.PlayNext`))
  ;[1 1 1] 播放sequencer
  (`/Engine/EditorBlueprintResources/StandardMacros.IsValid` _m_sequenceplayer
    (:`Is Valid`
      (`MovieSceneSequencePlayer.Play` _m_sequenceplayer)
      (`KismetSystemLibrary.PrintString` "aaaaaaaaaaaaaa"))))

(event `self.ReceiveTick`
  (params (DeltaSeconds :type "Float (single-precision)"))
  ;[1 1 1] 循环更新视角
)

(event `PlayOver`
  (bind _m_sequenceplayer (`self.m_sequencePlayer`))
  ;[1 1 1] 播放完一页暂停
  (`/Engine/EditorBlueprintResources/StandardMacros.IsValid` _m_sequenceplayer
    (:`Is Valid`
      (`MovieSceneSequencePlayer.Stop` _m_sequenceplayer))))

(event `CustomEvent`
  (params (DeltaSeconds :type "Float (double-precision)"))
  (bind _returnvalue (`WidgetLayoutLibrary.GetMousePositionOnViewport`))
  (`KismetSystemLibrary.PrintString` (`KismetStringLibrary.Conv_Vector2dToString` _returnvalue)))

(fn `GetPlayer`
  (returns (BGet :type Boolean))
  (bind _returnvalue (`GameplayStatics.GetActorOfClass` "/Game/FirstPersonCPP/Blueprints/FirstPersonCharacter.FirstPersonCharacter_C"))
  (`/Engine/EditorBlueprintResources/StandardMacros.IsValid` _returnvalue
    (:`Is Valid`
      (bind _asfirst_person_character (cast `/Game/FirstPersonCPP/Blueprints/FirstPersonCharacter` _returnvalue)
        (:`then`
          (set `self.Player` _asfirst_person_character)
          (return true))
        (:`CastFailed`
          _)))
    (:`Is Not Valid`
      _))
  (return false))

(fn `UserConstructionScript`)